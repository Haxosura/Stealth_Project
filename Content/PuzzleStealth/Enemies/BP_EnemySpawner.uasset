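; Enemy spawner actor that spawns an AI enemy once the player has been seen.
; Tick polls the cached player's PlayerSeen flag and, through a DoOnce, spawns a BP_EnenyAI at a random point in a flat box around the spawner.
; After a short delay the new enemy starts random movement.
; A ResetSpawner event re-arms the DoOnce for another spawn.
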(event `self.ReceiveBeginPlay`
  (bind _asbp_player (cast `/Game/PuzzleStealth/Player/BP_Player` (`GameplayStatics.GetPlayerCharacter` 0)))
  (set `self.BP Player` _asbp_player))

(event `self.ReceiveTick`
  (params (DeltaSeconds :type "Float (single-precision)"))
  (if (`/Game/PuzzleStealth/Player/BP_Player.Player Seen` (`self.BP Player`))
    (`/Engine/EditorBlueprintResources/StandardMacros.DoOnce` false :!label _label
      (:`Completed`
        (bind _returnvalue (`|SpawnActorFromClass` "/Game/PuzzleStealth/Enemies/BP_EnenyAI.BP_EnenyAI_C" (`KismetMathLibrary.MakeTransform` (`KismetMathLibrary.RandomPointInBoundingBox` (`self.K2_GetActorLocation`) (500.0 500.0 0.0))) "Undefined" "OverrideRootScale" null null))
        (`KismetSystemLibrary.Delay` 0.1)
        (`/Game/PuzzleStealth/Enemies/BP_EnenyAI.Random Movement` _returnvalue)))))

(event `ResetSpawner`
  (goto _label :!via `Reset`))

(fn `UserConstructionScript`)