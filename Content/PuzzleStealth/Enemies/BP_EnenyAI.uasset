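; Enemy AI pawn for a stealth game that roams random reachable points and chases the player unless they hide in a locker.
; Tick starts a looping roam once and issues a move toward the player every frame, regardless of sight, while the first BP_Locker found is not Hiding.
; DoOnce gates restart roaming when the player hides; PawnSensing sightings re-arm that restart and flag the player as AISeen.
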(event `self.ReceiveBeginPlay`
  (bind _asbp_player (cast `/Game/PuzzleStealth/Player/BP_Player` (`GameplayStatics.GetPlayerCharacter` 0)))
  (set `self.As BP Player` _asbp_player)
  (bind _returnvalue (`GameplayStatics.GetActorOfClass` "/Game/PuzzleStealth/Blueprints/BP_Locker.BP_Locker_C"))
  (set `self.BP Locker` _returnvalue))

(event `self.ReceiveTick`
  (params (DeltaSeconds :type "Float (single-precision)"))
  (`|ExecutionSequence`
    (:`then_0`
      (`/Engine/EditorBlueprintResources/StandardMacros.DoOnce` false :!label _label
        (:`Completed`
          (`KismetSystemLibrary.PrintString` "Moving")
          (`|AIMoveTo` self (`NavigationSystemV1.K2_GetRandomReachablePointInRadius` (`self.K2_GetActorLocation`) 1000.0 null null) null :!label _label_2
            (:`OnSuccess`
              (`KismetSystemLibrary.Delay` 0.2)
              (goto _label_2))))))
    (:`then_1`
      (`self.Chasing`))))

(event `Reset AI Movement`
  (goto _label :!via `Reset`))

(event `Chasing`
  (if (not (`/Game/PuzzleStealth/Blueprints/BP_Locker.Hiding` (`self.BP Locker`)))
    (`|AIMoveTo` self (`self.K2_GetActorLocation`) (`self.As BP Player`))
    (else
      (`/Engine/EditorBlueprintResources/StandardMacros.DoOnce` false :!label _label_3
        (:`Completed`
          (`self.Reset AI Movement`))))))

(event `self.PawnSensing.OnSeePawn`
  (params (Pawn :type "Pawn Object Reference"))
  (set `/Game/PuzzleStealth/Player/BP_Player.Pawn` Pawn (`self.As BP Player`))
  (`|ExecutionSequence`
    (:`then_0`
      (goto _label_3 :!via `Reset`))
    (:`then_1`
      (set `/Game/PuzzleStealth/Player/BP_Player.AI Seen` true (`self.As BP Player`))
      (`KismetSystemLibrary.PrintString` "AI Seen"))))

(fn `Crouch Trace Distance`
  (params (`Trace Distances` :type "Float (double-precision)") (DrawDebugType :type "EDrawDebugTrace Enum" :default "None"))
  (bind _returnvalue (`SceneComponent.K2_GetComponentLocation` (`self.CapsuleComponent`)))
  (bind _outhit (`KismetSystemLibrary.LineTraceSingle` _returnvalue (+ _returnvalue (`KismetMathLibrary.MakeVector` 0.0 0.0 `Trace Distances`)) "TraceTypeQuery1" false (`|MakeArray` self :!type "Actor Object Reference") DrawDebugType))
  (if (`GameplayStatics.BreakHitResult` _outhit)
    _))

(fn `UserConstructionScript`)