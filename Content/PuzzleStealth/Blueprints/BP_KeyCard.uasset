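; Key card pickup for the puzzle stealth game that grants the player the card identified by its CardNum.
; On BeginPlay it enables input from the first player controller and caches the BP_Player character.
; The PlayerPickUp event sets that index in the player's KeyCards array to true, then destroys the actor.
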(event `self.ReceiveBeginPlay`
  (`self.EnableInput` self (`GameplayStatics.GetPlayerController` 0))
  (bind _asbp_player (cast `/Game/PuzzleStealth/Player/BP_Player` (`GameplayStatics.GetPlayerCharacter` 0)))
  (set `self.BP Player` _asbp_player))

(event `Player PickUp`
  (`KismetArrayLibrary.Array_Set` (`/Game/PuzzleStealth/Player/BP_Player.KeyCards` (`self.BP Player`)) (`self.CardNum`) true)
  (`self.K2_DestroyActor`))

(fn `UserConstructionScript`)