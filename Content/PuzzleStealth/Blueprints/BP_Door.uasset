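; BP_Door is a keycard-locked door that slides its Cube vertically when the player approaches.
; Overlapping CardCollision with the required card in BP_Player's KeyCards sets KeyCardUsed and plays a timeline driving the Cube's relative Z.
; That timeline's play and reverse are each limited by a DoOnce.
; Once KeyCardUsed is set, OpenCollision overlaps play and reverse a second timeline on the same Cube.
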(event `self.CardCollision.OnComponentBeginOverlap`
  (params (OverlappedComponent :type "PrimitiveComponent Object Reference") (OtherActor :type "Actor Object Reference") (OtherComp :type "PrimitiveComponent Object Reference") (OtherBodyIndex :type Integer) (bFromSweep :type Boolean) (SweepResult :type "HitResult Structure (by ref)"))
  (bind _asbp_player (cast `/Game/PuzzleStealth/Player/BP_Player` OtherActor))
  (if (`|GetArrayItem` (`/Game/PuzzleStealth/Player/BP_Player.KeyCards` _asbp_player) (`self.Card Needed`))
    (`KismetSystemLibrary.PrintString` "Hello")
    (set `self.KeyCardUsed` true)
    (`/Engine/EditorBlueprintResources/StandardMacros.DoOnce` false
      (:`Completed`
        (bind (_direction _aphla) (`Timeline|Timeline` :!label _label)
          (:`Update`
            (`SceneComponent.K2_SetRelativeLocation` (`self.Cube`) (`KismetMathLibrary.MakeVector` 0.0 0.0 _aphla) false false)))))))

(event `self.CardCollision.OnComponentEndOverlap`
  (params (OverlappedComponent :type "PrimitiveComponent Object Reference") (OtherActor :type "Actor Object Reference") (OtherComp :type "PrimitiveComponent Object Reference") (OtherBodyIndex :type Integer))
  (cast `/Game/PuzzleStealth/Player/BP_Player` OtherActor)
  (`/Engine/EditorBlueprintResources/StandardMacros.DoOnce` false
    (:`Completed`
      (goto _label :!via `Reverse`))))

(event `self.OpenCollision.OnComponentBeginOverlap`
  (params (OverlappedComponent :type "PrimitiveComponent Object Reference") (OtherActor :type "Actor Object Reference") (OtherComp :type "PrimitiveComponent Object Reference") (OtherBodyIndex :type Integer) (bFromSweep :type Boolean) (SweepResult :type "HitResult Structure (by ref)"))
  (cast `/Game/PuzzleStealth/Player/BP_Player` OtherActor)
  (if (`self.KeyCardUsed`)
    (bind (_direction _aphla) (`Timeline|OpenDoor` :!label _label_2)
      (:`Update`
        (`SceneComponent.K2_SetRelativeLocation` (`self.Cube`) (`KismetMathLibrary.MakeVector` 0.0 0.0 _aphla) false false)))))

(event `self.OpenCollision.OnComponentEndOverlap`
  (params (OverlappedComponent :type "PrimitiveComponent Object Reference") (OtherActor :type "Actor Object Reference") (OtherComp :type "PrimitiveComponent Object Reference") (OtherBodyIndex :type Integer))
  (cast `/Game/PuzzleStealth/Player/BP_Player` OtherActor)
  (if (`self.KeyCardUsed`)
    (goto _label_2 :!via `Reverse`)))

(fn `UserConstructionScript`)