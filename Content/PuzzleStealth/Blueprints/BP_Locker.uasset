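; BP_Locker is an interactable hiding spot the player enters or leaves by pressing E.
; Collision box overlaps enable or disable input and open or close a gate on the key press.
; ToggleHide flips the player's visibility and collision, blending the camera to the locker or back to the player.
; Each use also replays a timeline that swings the door yaw between open and close angles.
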(event `self.ReceiveBeginPlay`
  (`self.EnableInput` (`GameplayStatics.GetPlayerController` 0))
  (bind _asbp_player (cast `/Game/PuzzleStealth/Player/BP_Player` (`GameplayStatics.GetPlayerCharacter` 0)))
  (set `self.BP Player` _asbp_player))

(event `Key|E`
  (params (Key :type "Key Structure"))
  (:`Pressed`
    (`/Engine/EditorBlueprintResources/StandardMacros.Gate` true :!label _label
      (:`Exit`
        (`|ExecutionSequence`
          (:`then_0`
            (`self.Toggle Hide`)
            (`KismetSystemLibrary.Delay` 1.0)
            (`self.EnableInput` (`GameplayStatics.GetPlayerController` 0) :!label _label_2)
            (goto _label :!via `Open`))
          (:`then_1`
            (bind (_direction _door_track) (`Timeline|LockerDoor` :!via `PlayFromStart`)
              (:`Update`
                (`SceneComponent.K2_SetRelativeRotation` (`self.Door`) (`KismetMathLibrary.MakeRotator` 0.0 0.0 (`KismetMathLibrary.Lerp` (`self.Open Angle`) (`self.Close Angle`) _door_track)) false false)))))))))

(event `self.CollisonBox.OnComponentBeginOverlap`
  (params (OverlappedComponent :type "PrimitiveComponent Object Reference") (OtherActor :type "Actor Object Reference") (OtherComp :type "PrimitiveComponent Object Reference") (OtherBodyIndex :type Integer) (bFromSweep :type Boolean) (SweepResult :type "HitResult Structure (by ref)"))
  (cast `/Game/PuzzleStealth/Player/BP_Player` OtherActor)
  (goto _label_2))

(event `self.CollisonBox.OnComponentEndOverlap`
  (params (OverlappedComponent :type "PrimitiveComponent Object Reference") (OtherActor :type "Actor Object Reference") (OtherComp :type "PrimitiveComponent Object Reference") (OtherBodyIndex :type Integer))
  (cast `/Game/PuzzleStealth/Player/BP_Player` OtherActor)
  (`self.DisableInput` (`GameplayStatics.GetPlayerController` 0))
  (goto _label :!via `Close`))

(fn `Toggle Hide`
  (bind _returnvalue (`GameplayStatics.GetPlayerController` 0))
  (bind _bp_player (`self.BP Player`))
  (if (`self.Hiding`)
    (set `self.Hiding` false)
    (`self.SetActorHiddenInGame` _bp_player false)
    (`self.SetActorEnableCollision` _bp_player true)
    (`PlayerController.SetViewTargetWithBlend` _returnvalue _bp_player 0.6 "VTBlend_Linear" 0.0 false)
    (else
      (set `self.Hiding` true)
      (`self.SetActorHiddenInGame` _bp_player true)
      (`self.SetActorEnableCollision` _bp_player false)
      (`PlayerController.SetViewTargetWithBlend` _returnvalue self 0.6 "VTBlend_Linear" 0.0 false))))

(fn `UserConstructionScript`)